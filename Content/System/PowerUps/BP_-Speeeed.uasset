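; Speed power-up actor that triggers Speeeed on the ThirdPersonCharacter and destroys itself when touched.
; A timeline started on BeginPlay animates its position as an offset from InitialLocation, which is captured once on the first Tick rather than in BeginPlay.
; Box overlap casts to both Pollution and ThirdPersonCharacter into shared destroy and Speeeed calls, though the Pollution branch never sets the character reference it uses.
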(event `self.ReceiveBeginPlay`
  (bind (_direction _newtrack_0) (`Timeline|Timeline_0`)
    (:`Update`
      (`self.K2_SetActorLocation` (+ _newtrack_0 (`self.Initial_location`))))))

(event `self.ReceiveTick`
  (params (DeltaSeconds :type "Float (single-precision)"))
  (`/Engine/EditorBlueprintResources/StandardMacros.DoOnce` false
    (:`Completed`
      (set `self.Initial_location` (`self.K2_GetActorLocation`)))))

(event `self.Box.OnComponentBeginOverlap`
  (params (OverlappedComponent :type "PrimitiveComponent Object Reference") (OtherActor :type "Actor Object Reference") (OtherComp :type "PrimitiveComponent Object Reference") (OtherBodyIndex :type Integer) (bFromSweep :type Boolean) (SweepResult :type "HitResult Structure (by ref)"))
  (`|ExecutionSequence`
    (:`then_0`
      (cast `/Game/Shootingassets/Projectiles/Pollution` OtherActor)
      (`|ExecutionSequence`
        (:`then_0`
          (`self.K2_DestroyActor` :!label _label))
        (:`then_1`
          (`/Game/Characters/ThirdPerson/ThirdPersonBP/Blueprints/ThirdPersonCharacter.Speeeed` (stale _asthird_person_character) :!label _label_2))))
    (:`then_1`
      (bind _asthird_person_character (cast `/Game/Characters/ThirdPerson/ThirdPersonBP/Blueprints/ThirdPersonCharacter` OtherActor))
      (`|ExecutionSequence`
        (:`then_0`
          (goto _label))
        (:`then_1`
          (goto _label_2))))))

(fn `UserConstructionScript`)